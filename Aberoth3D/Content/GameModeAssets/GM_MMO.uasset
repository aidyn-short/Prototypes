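; GM_MMO is a game mode Blueprint that keeps an object pool of BP_AICharacter enemies.
; On BeginPlay it pre-spawns characters based on Minimum at a far-off location, hidden with collision and tick disabled, and stores them in Inactive.
; GetInactive moves the last Inactive entry into Active and returns it, without re-enabling it or checking for an empty pool.
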(event EventBeginPlay
  (for _index (range 0 (Variables|Default|GetMinimum))
    (bind _returnvalue (Game|SpawnActorfromClass "/Game/Enemies/BP_AICharacter.BP_AICharacter_C" (Math|Transform|MakeTransform "50000.000000,50000.000000,-50000.000000" "0, 0, 0" "1.000000,1.000000,1.000000") "AlwaysSpawn" "MultiplyWithRoot" 0 0))
    (Rendering|SetActorHiddenInGame _returnvalue true)
    (Collision|SetActorEnableCollision _returnvalue false)
    (Actor|Tick|SetActorTickEnabled _returnvalue)
    (Utilities|Array|Add (Variables|Default|GetInactive) _returnvalue)))

(fn ConstructionScript)

(fn GetInactive
  (bind _inactive (Variables|Default|GetInactive))
  (bind _returnvalue (Utilities|Array|Length _inactive))
  (bind _returnvalue_2 (- _returnvalue 1))
  (bind _output (Utilities|Array|Get(acopy) _inactive _returnvalue_2))
  (bind _output_get (LocalVariables|SetEnemyToPass _output))
  (Utilities|Array|Add (Variables|Default|GetActive) _output)
  (Utilities|Array|Resize _inactive _returnvalue_2)
  (return _output_get))
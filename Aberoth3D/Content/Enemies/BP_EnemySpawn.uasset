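; BP_EnemySpawn is an enemy spawn point that populates the area around itself from a pool held by the GM_MMO game mode.
; One second after BeginPlay it takes inactive enemies up to MaxCount, setting each up with EnemyType.
; It teleports each to a random reachable navmesh point within SpawnRadius and records itself as that enemy's Spawn.
; The SpawnEnemy function is an empty stub.
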(event EventBeginPlay
  (bind _returnvalue (Transformation|GetActorLocation))
  (bind _spawnradius (Variables|Default|GetSpawnRadius))
  (bind _randomlocation (AI|Navigation|GetRandomReachablePointinRadius _returnvalue _spawnradius 0 0))
  (Utilities|FlowControl|Delay 1.0)
  (bind _asgm_mmo (Utilities|Casting|CastToGM_MMO (Game|GetGameMode)))
  (bind _output_get (Variables|Default|SetGameMode _asgm_mmo))
  (for _index (range 1 (Variables|Default|GetMaxCount))
    (bind _inactiveenemy (Default|GetInactive _output_get))
    (Default|SpawnSetUp _inactiveenemy (Variables|Default|GetEnemyType))
    (Transformation|SetActorLocation _inactiveenemy (Math|Vector|MakeVector (.x _randomlocation) (.y _randomlocation) (.z _randomlocation)) false true)
    (Variables|/Game/Enemies/BP_AICharacter.BP_AICharacter_C|SetSpawn _inactiveenemy self)))

(fn ConstructionScript)

(fn SpawnEnemy)
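; Player punch gameplay ability that deals damage to a target in front of the character.
; On authority only, it sphere-traces from the avatar's location along the control rotation, with persistent debug drawing.
; If the hit actor has an ability system component, it applies GE_Damage and prints one of that target's attribute values.
; EndAbility is called only on the authority path, after a successful character cast.
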(event Ability|EventActivateAbility
  (bind _returnvalue (Ability|GetAvatarActorfromActorInfo))
  (bind _returnvalue_2 (Transformation|GetActorLocation _returnvalue))
  (Ability|HasAuthority
    (:True
      (bind _asbp_mmocharacter (Utilities|Casting|CastToBP_MMOCharacter _returnvalue))
      (bind _outhit (Collision|SphereTraceForObjects _returnvalue_2 (+ _returnvalue_2 (* (Math|Vector|GetForwardVector (Pawn|GetControlRotation _asbp_mmocharacter :!class /Script/Engine.Pawn)) 5e+02)) 1e+01 (Utilities|Array|MakeArray "ObjectTypeQuery9") false 0 "Persistent"))
      (Utilities|IsValid (Ability|GetAbilitySystemComponent (.hitactor _outhit))
        (:Is%20Valid
          (GameplayEffects|ApplyGameplayEffectToTarget (Ability|TargetData|AbilityTargetDatafromActor (.hitactor _outhit)) "/Game/GAS/Effects/GE_Damage.GE_Damage_C" 1 1)
          (Development|PrintString (Utilities|String|ToString(Float) (.ReturnValue (Class|AbilitySystemComponent|GetGameplayAttributeValue (Ability|GetAbilitySystemComponent (.hitactor _outhit)) "(AttributeName=\"Health\",Attribute=/Script/Aberoth3D.GeneralAttributeSet:Health,AttributeOwner=\"/Script/CoreUObject.Class'/Script/Aberoth3D.GeneralAttributeSet'\")")))))
        (:Is%20Not%20Valid
          _))
      (Ability|EndAbility))))
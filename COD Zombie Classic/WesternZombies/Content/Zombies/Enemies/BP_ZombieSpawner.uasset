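; Zombie spawner that places one NPC of a configurable class at its spawn capsule and respawns it after death.
; BeginPlay spawns the first NPC after an initial delay if immediate spawning is enabled; otherwise nothing in this graph calls SpawnEnemy.
; Each spawn binds to the NPC's OnDeath event, which decrements SpawnCount and, while any remain, spawns again after a retriggerable delay.
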(event Custom|Spawn%20Enemy
  ;[1 1 1] NPC Spawning
  ;;[1 1 1] Spawn the NPC. If you implement more NPC types, you can change the type spawned by changing the NPC Class variable.
  (bind _returnvalue (Game|SpawnActorfromClass (Variables|Spawner|GetNPC%20Class) (Transformation|GetWorldTransform (Variables|Default|GetSpawn%20Capsule)) "AdjustIfPossibleButAlwaysSpawn" "MultiplyWithRoot" 0 0))
  ;;[1 1 1] Listen for the NPC death event
  (EventDispatchers|BindEventtoOnDeath _returnvalue (EventDispatchers|CreateEvent :!event Custom|On%20NPC%20Died)))

(event Custom|On%20NPC%20Died
  ;[1 1 1] NPC Death and Respawn
  ;;[1 1 1] Do we still have NPCs left to spawn?
  (bind _result (Math|Integer|DecrementInt (Variables|Spawner|GetSpawn%20Count))
    (:%20%20
      (if (not (<= _result 0))
        ;;[1 1 1] Wait for a bit and respawn
        (Utilities|FlowControl|RetriggerableDelay (Variables|Spawner|GetRespawn%20Delay))
        (CallFunction|SpawnEnemy)))))

(event EventBeginPlay
  ;[1 1 1] Spawner Initialization
  ;;[1 1 1] Should we spawn the first NPC immediately?
  (if (Variables|Spawner|GetShould%20Spawn%20Enemies%20Immediately)
    ;;[1 1 1] Wait for a bit and spawn the first NPC.
    (Utilities|FlowControl|Delay (Variables|Spawner|GetInitial%20Spawn%20Delay))
    (CallFunction|SpawnEnemy)))

(fn ConstructionScript)
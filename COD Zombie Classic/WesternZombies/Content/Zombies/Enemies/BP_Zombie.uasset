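; BP_Zombie is an enemy zombie character that tracks its own health and handles its death.
; Incoming damage lowers CurrentHP, and the killing hit stops the StateTree logic on its BP_ZombieController before calling Die.
; Die disables movement and capsule collision, notifies the SpawnManager, then plays the dying montage and destroys the actor when it blends out.
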(event Custom|Die
  (bind _charactermovement (Variables|Character|GetCharacterMovement))
  ;[1 1 1] Death handling
  (Utilities|FlowControl|Sequence
    (:then_0
      (Components|Movement|StopMovementImmediately _charactermovement)
      (Pawn|Components|CharacterMovement|DisableMovement _charactermovement)
      (Collision|SetCollisionEnabled (Variables|Collision|GetCapsuleComponent) "NoCollision"))
    (:then_1
      (Default|ZombieDied (Variables|Default|GetSpawnManager)))
    (:then_2
      (Animation|Montage|PlayMontage (Variables|Character|GetMesh) "/Game/Zombies/Enemies/Mixamo/Zombie_Dying_Montage.Zombie_Dying_Montage"
        (:OnBlendOut
          (Actor|DestroyActor))))))

(event Collision|EventActorBeginOverlap
  (params (OtherActor :type Actor%20Object%20Reference)))

(event EventTick
  (params (DeltaSeconds :type Float%20%28single-precision%29)))

(event Game|Damage|EventAnyDamage
  (params (Damage :type Float%20%28single-precision%29) (DamageType :type Damage%20Type%20Object%20Reference) (InstigatedBy :type Controller%20Object%20Reference) (DamageCauser :type Actor%20Object%20Reference))
  (if (> (Variables|Default|GetCurrent%20HP) 0.0)
    (bind _output_get (Variables|Default|SetCurrent%20HP (- (Variables|Default|GetCurrent%20HP) Damage)))
    (if (<= _output_get 0.0)
      (bind _asbp_zombie_controller (Utilities|Casting|CastToBP_ZombieController (Pawn|GetController self)))
      (AI|Logic|StopLogic (Variables|/Game/Zombies/Enemies/BP_ZombieController.BP_ZombieController_C|GetStateTreeAI _asbp_zombie_controller) "death")
      (CallFunction|Die))))

(fn ConstructionScript)